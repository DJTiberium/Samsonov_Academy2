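; Game mode Blueprint that sets up the player UI and keeps a running score.
; On BeginPlay it creates the HUD widget and adds it to the viewport.
; The ScoreCount event adds an incoming amount to TotalScore.
; The Deployment event opens the DeployMenu widget for player controller 0 and shows the mouse cursor, without changing the input mode.
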(event Custom|ScoreCount
  (params (AddScore :type Integer))
  (Variables|Default|SetTotalScore (+ AddScore (Variables|Default|GetTotalScore))))

(event Custom|Deployment
  (bind _returnvalue (Game|GetPlayerController 0))
  (bind _returnvalue_2 (UserInterface|CreateWidget "/Game/Blueprints/MainCharacter/Widgets/DeployMenu.DeployMenu_C" _returnvalue))
  (UserInterface|Viewport|AddtoViewport _returnvalue_2 0)
  (Variables|/Script/Engine.PlayerController|SetbShowMouseCursor _returnvalue true))

(event EventBeginPlay
  (bind _returnvalue (UserInterface|CreateWidget "/Game/Blueprints/MainCharacter/Widgets/HUD.HUD_C"))
  (UserInterface|Viewport|AddtoViewport _returnvalue 0))

(fn ConstructionScript)