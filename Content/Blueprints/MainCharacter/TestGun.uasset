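; TestGun is an actor that fires continuously on its own from BeginPlay, apparently as a weapon test.
; A looping Delay sets the fire interval, and each cycle spawns a Bullet303B at the Arrow component's transform with a random yaw offset bounded by Spray.
; Each shot also spawns an emitter at the ParticleSystem component and plays two sounds at the actor's location.
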(event EventBeginPlay
  (bind _returnvalue (Transformation|GetActorLocation))
  (bind _arrow (Variables|Default|GetArrow))
  (bind _spray (Variables|Default|GetSpray))
  (bind _particlesystem (Variables|Default|GetParticleSystem))
  (bind _returnvalue_2 (Transformation|GetWorldTransform _arrow))
  (bind (_location _rotation _scale) (Math|Transform|BreakTransform _returnvalue_2))
  (Utilities|FlowControl|Delay (Variables|Default|GetDuration) :!label _label)
  (Game|SpawnActorfromClass "/Game/Blueprints/Weapons/Bullet/Bullet-303B.Bullet-303B_C" (Math|Transform|MakeTransform _location (Math|Rotator|Delta(Rotator) _rotation (Math|Rotator|MakeRotator 0.0 0.0 (Math|Random|RandomFloatinRange (* _spray -1.0) _spray))) _scale) "Undefined" 0 0)
  (Effects|SpawnEmitteratLocation "/Game/Realistic_Starter_VFX_Pack_Vol2/Particles/Hit/P_Default.P_Default" (Transformation|GetSocketLocation _particlesystem "None") (Transformation|GetSocketRotation _particlesystem "None"))
  (Audio|PlaySoundatLocation (Variables|Default|GetSound_0) _returnvalue "0, 0, 0" 1.0 1.0 0.0 0 0 0)
  (Audio|PlaySoundatLocation (Variables|Default|GetSound) _returnvalue "0, 0, 0" 1.0 1.0 0.0 0 0 0)
  (goto _label))

(event Collision|EventActorBeginOverlap
  (params (OtherActor :type Actor%20Object%20Reference)))

(event EventTick
  (params (DeltaSeconds :type Float%20%28single-precision%29)))

(fn ConstructionScript)