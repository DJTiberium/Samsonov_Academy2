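; MainController is the player controller that owns the HUD and switches its screens for the controlled MainCharacter.
; On begin play it creates the HUD and caches the pawn.
; Each tick it shows interaction text for weapons, military depots or heavily wounded teammates, and polls wounded and dead states to open their screens.
; Those screens and the WeaponChoice event enable the cursor and UI-only input.
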(event Custom|WeaponChoice
  (bind _self self)
  (bind _hudref (Variables|Default|GetHUDref))
  (Class|WidgetSwitcher|SetActiveWidgetIndex (Variables|/Game/Blueprints/MainCharacter/Widgets/HUD.HUD_C|GetMainSwitcher _hudref) 3)
  (Variables|/Script/Engine.PlayerController|SetbShowMouseCursor _self true)
  (Input|SetInputModeUIOnly _self _hudref "DoNotLock"))

(event EventBeginPlay
  (Utilities|FlowControl|Sequence
    (:then_0
      (bind _returnvalue (UserInterface|CreateWidget "/Game/Blueprints/MainCharacter/Widgets/HUD.HUD_C" self))
      (Variables|Default|SetHUDref _returnvalue)
      (UserInterface|Viewport|AddtoViewport (Variables|Default|GetHUDref) 0))
    (:then_1
      (bind _asmain_character (Utilities|Casting|CastToMainCharacter (Pawn|GetControlledPawn)))
      (Variables|Default|SetPawnRef _asmain_character))))

(event EventTick
  (params (DeltaSeconds :type Float%20%28single-precision%29))
  (bind _returnvalue (Game|GetPlayerController 0))
  (bind _returnvalue_2 (Game|GetPlayerController 0))
  (if (Utilities|IsValid (Variables|Default|GetPawnRef))
    (Utilities|FlowControl|Sequence
      (:then_0
        (|InteractInfo))
      (:then_1
        (if (Variables|/Game/Blueprints/MainCharacter/MainCharacter.MainCharacter_C|GetIsHeavyWounded (Variables|Default|GetPawnRef))
          (Variables|Default|SetIsAlive false)
          (Class|WidgetSwitcher|SetActiveWidgetIndex (Variables|/Game/Blueprints/MainCharacter/Widgets/HUD.HUD_C|GetMainSwitcher (Variables|Default|GetHUDref)) 1)
          (bind _asmain_controller (Utilities|Casting|CastToMainController _returnvalue_2))
          (Variables|/Script/Engine.PlayerController|SetbShowMouseCursor _asmain_controller true)
          (Input|SetInputModeUIOnly _returnvalue_2 0 "DoNotLock")))
      (:then_2
        (if (Variables|/Game/Blueprints/MainCharacter/MainCharacter.MainCharacter_C|GetIsDead (Variables|Default|GetPawnRef))
          (Variables|Default|SetIsAlive false)
          (Class|WidgetSwitcher|SetActiveWidgetIndex (Variables|/Game/Blueprints/MainCharacter/Widgets/HUD.HUD_C|GetMainSwitcher (Variables|Default|GetHUDref)) 2)
          (bind _asmain_controller_2 (Utilities|Casting|CastToMainController _returnvalue))
          (Variables|/Script/Engine.PlayerController|SetbShowMouseCursor _asmain_controller_2 true)
          (Input|SetInputModeUIOnly _returnvalue 0 "DoNotLock"))))))

(fn ConstructionScript)